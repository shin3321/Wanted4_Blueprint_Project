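; BP_Huntress is the player-controlled Huntress character, with Enhanced Input for look, movement, melee attack, axe throw and carrying.
; A HunterState enum gates actions, while delays and walk-speed changes slow her during wind-up and root her during attacks and throws.
; Throw only changes state and speed here, with no projectile spawned.
; Once UpPlayer enables carrying, the carry input hides the axe and passes her mesh to BP_FengMin's Interact.
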(event `self.ReceiveBeginPlay`
  (set `self.DefaultSpeed` (`CharacterMovementComponent.MaxWalkSpeed` (`self.CharacterMovement`))))

(event `EnhancedInput|/Game/Blueprint/FengMin/FengMinController/IA_Rotation`
  (params (ActionValue :type "Vector2D Structure") (ElapsedSeconds :type "Float (double-precision)") (TriggeredSeconds :type "Float (double-precision)") (InputAction :type "InputAction Object Reference" :default "/Game/Blueprint/FengMin/FengMinController/IA_Rotation.IA_Rotation"))
  ; Rotation
  (:`Triggered`
    (`self.AddControllerYawInput` ActionValue_X)
    (`self.AddControllerPitchInput` ActionValue_Y)))

(event `EnhancedInput|/Game/Blueprint/Huntress/HuntressController/IA_Attack`
  (params (ActionValue :type Boolean) (ElapsedSeconds :type "Float (double-precision)") (TriggeredSeconds :type "Float (double-precision)") (InputAction :type "InputAction Object Reference" :default "/Game/Blueprint/Huntress/HuntressController/IA_Attack.IA_Attack"))
  ; Attack
  (:`Triggered`
    (switch `/Game/Blueprint/Huntress/EHunterState` (`self.HunterState`)
      (:`NewEnumerator0`
        (set `self.HunterState` "NewEnumerator5")
        (`self.PlayAnimMontage` "/Game/Blueprint/Huntress/Animation/AM_HuntressAttack.AM_HuntressAttack")
        (set `CharacterMovementComponent.MaxWalkSpeed` 0.0 (`self.CharacterMovement`))
        (`KismetSystemLibrary.Delay` 1.5)
        (set `CharacterMovementComponent.MaxWalkSpeed` (`self.DefaultSpeed`) (`self.CharacterMovement`)))
      (:`NewEnumerator4`
        (set `self.HunterState` "NewEnumerator0")
        (set `CharacterMovementComponent.MaxWalkSpeed` (`self.DefaultSpeed`) (`self.CharacterMovement`))))))

(event `EnhancedInput|/Game/Blueprint/FengMin/FengMinController/IA_Move`
  (params (ActionValue :type "Vector2D Structure") (ElapsedSeconds :type "Float (double-precision)") (TriggeredSeconds :type "Float (double-precision)") (InputAction :type "InputAction Object Reference" :default "/Game/Blueprint/FengMin/FengMinController/IA_Move.IA_Move"))
  (bind (_returnvalue_roll _returnvalue_pitch _returnvalue_yaw) (`KismetMathLibrary.BreakRotator` (`self.GetControlRotation`)))
  ; Movement
  (:`Triggered`
    (switch `/Game/Blueprint/Huntress/EHunterState` (`self.HunterState`)
      (:`NewEnumerator0`
        _)
      (:`NewEnumerator3`
        _)
      (:`NewEnumerator4`
        _))
    (`self.AddMovementInput` (`KismetMathLibrary.GetRightVector` (`self.GetControlRotation`)) ActionValue_X)
    (`self.AddMovementInput` (`KismetMathLibrary.GetForwardVector` (`KismetMathLibrary.MakeRotator` 0.0 0.0 _returnvalue_yaw)) ActionValue_Y)))

(event `EnhancedInput|/Game/Blueprint/Huntress/HuntressController/IA_Throw`
  (params (ActionValue :type Boolean) (ElapsedSeconds :type "Float (double-precision)") (TriggeredSeconds :type "Float (double-precision)") (InputAction :type "InputAction Object Reference" :default "/Game/Blueprint/Huntress/HuntressController/IA_Throw.IA_Throw"))
  ; Throw
  (:`Started`
    (if (`|EnumEquality` (`self.HunterState`) "NewEnumerator0")
      (set `self.HunterState` "NewEnumerator3")
      (set `CharacterMovementComponent.MaxWalkSpeed` (* (`self.DefaultSpeed`) 0.7) (`self.CharacterMovement`))))
  (:`Completed`
    (set `self.HunterState` "NewEnumerator4")
    (set `CharacterMovementComponent.MaxWalkSpeed` 0.0 (`self.CharacterMovement`))
    (`KismetSystemLibrary.Delay` 1.5)
    (set `self.HunterState` "NewEnumerator0")
    (set `CharacterMovementComponent.MaxWalkSpeed` (`self.DefaultSpeed`) (`self.CharacterMovement`))))

(event `AttackBegin`)

(event `AttackEnd`
  (set `self.HunterState` "NewEnumerator0"))

(event `UpPlayer`
  (set `self.CanCarry` true))

(event `EnhancedInput|/Game/Blueprint/Huntress/HuntressController/IA_Carry`
  (params (ActionValue :type Boolean) (ElapsedSeconds :type "Float (double-precision)") (TriggeredSeconds :type "Float (double-precision)") (InputAction :type "InputAction Object Reference" :default "/Game/Blueprint/Huntress/HuntressController/IA_Carry.IA_Carry"))
  (:`Triggered`
    (if (`self.CanCarry`)
      (set `self.HunterState` "NewEnumerator6")
      (`SceneComponent.SetVisibility` (`self.Axe`) false false)
      (bind _asbp_feng_min (cast `/Game/Blueprint/FengMin/BP_FengMin` (`self.CarryOnPlayer`)))
      (`/Game/Blueprint/FengMin/BP_FengMin.Interact` _asbp_feng_min (`self.Mesh`)))))

(fn `UserConstructionScript`)