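; Player character Blueprint for Feng Min, a survivor who can be downed, carried and hooked by BP_Huntress, with Enhanced Input for look, move and run.
; A first hit injures her with a brief speed burst; a second downs her and enables FaintCollision.
; That overlap calls the Huntress's UpPlayer, and Interact attaches her to a carry socket.
; LifttoHook attaches to an overlapped BP_Hook, notifying it when HookNum is below three.
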(event `self.ReceiveBeginPlay`
  (set `self.DefaultSpeed` (`CharacterMovementComponent.MaxWalkSpeed` (`self.CharacterMovement`)))
  (`PrimitiveComponent.SetCollisionEnabled` (`self.FaintCollision`) "NoCollision"))

(event `EnhancedInput|/Game/Blueprint/Controller/IA_Rotation`
  (params (ActionValue :type "Vector2D Structure") (ElapsedSeconds :type "Float (double-precision)") (TriggeredSeconds :type "Float (double-precision)") (InputAction :type "InputAction Object Reference" :default "/Game/Blueprint/Controller/IA_Rotation.IA_Rotation"))
  ; Rotation
  (:`Triggered`
    (`self.AddControllerYawInput` ActionValue_X)
    (`self.AddControllerPitchInput` ActionValue_Y)))

(event `EnhancedInput|/Game/Blueprint/Controller/IA_Move`
  (params (ActionValue :type "Vector2D Structure") (ElapsedSeconds :type "Float (double-precision)") (TriggeredSeconds :type "Float (double-precision)") (InputAction :type "InputAction Object Reference" :default "/Game/Blueprint/Controller/IA_Move.IA_Move"))
  (bind (_returnvalue_roll _returnvalue_pitch _returnvalue_yaw) (`KismetMathLibrary.BreakRotator` (`self.GetControlRotation`)))
  ; Movement
  (:`Triggered`
    (`self.AddMovementInput` (`KismetMathLibrary.GetRightVector` (`self.GetControlRotation`)) ActionValue_X)
    (`self.AddMovementInput` (`KismetMathLibrary.GetForwardVector` (`KismetMathLibrary.MakeRotator` 0.0 0.0 _returnvalue_yaw)) ActionValue_Y)))

(event `EnhancedInput|/Game/Blueprint/Controller/IA_Run`
  (params (ActionValue :type Boolean) (ElapsedSeconds :type "Float (double-precision)") (TriggeredSeconds :type "Float (double-precision)") (InputAction :type "InputAction Object Reference" :default "/Game/Blueprint/Controller/IA_Run.IA_Run"))
  ; Run
  (:`Triggered`
    (set `CharacterMovementComponent.MaxWalkSpeed` (`self.RunSpeed`) (`self.CharacterMovement`))
    (set `self.PlayerStatee` "NewEnumerator6")))

(event `GetAttacked`
  (bind _charactermovement (`self.CharacterMovement`))
  ; 공격 받은 후 로직 처리
  (if (`self.PlayerInjured`)
    (set `self.PlayerStatee` "NewEnumerator17")
    (set `CharacterMovementComponent.MaxWalkSpeed` (`self.FaintSpeed`) (`self.CharacterMovement`))
    (`PrimitiveComponent.SetCollisionEnabled` (`self.FaintCollision`) "QueryOnly")
    (else
      (set `self.PlayerInjured` true)
      (set `CharacterMovementComponent.MaxWalkSpeed` (* (`self.RunSpeed`) 1.3) _charactermovement)
      (`KismetSystemLibrary.Delay` 1.5)
      (set `CharacterMovementComponent.MaxWalkSpeed` (`self.RunSpeed`) _charactermovement))))

(event `self.FaintCollision.OnComponentBeginOverlap`
  (params (OverlappedComponent :type "PrimitiveComponent Object Reference") (OtherActor :type "Actor Object Reference") (OtherComp :type "PrimitiveComponent Object Reference") (OtherBodyIndex :type Integer) (bFromSweep :type Boolean) (SweepResult :type "HitResult Structure (by ref)"))
  (bind _asbp_huntress (cast `/Game/Blueprint/Huntress/BP_Huntress` OtherActor))
  (if true
    (set `/Game/Blueprint/Huntress/BP_Huntress.CarryOnPlayer` self _asbp_huntress)
    (`/Game/Blueprint/Huntress/BP_Huntress.UpPlayer` _asbp_huntress)))

(event `/Game/Blueprint/Huntress/BI_CarryPlayer.Interact`
  (params (NewParaParentMeshm :type "SkeletalMeshComponent Object Reference"))
  (if (`|EnumEquality` (`self.PlayerStatee`) "NewEnumerator17")
    (set `self.PlayerStatee` "NewEnumerator13")
    (`PrimitiveComponent.SetCollisionEnabled` (`self.FaintCollision`) "NoCollision")
    (`PrimitiveComponent.SetCollisionEnabled` (`self.CapsuleComponent`) "NoCollision")
    (`self.K2_AttachToComponent` NewParaParentMeshm "PlayerCarrySocket" "SnapToTarget" "SnapToTarget" "KeepRelative")))

(event `/Game/Blueprint/Huntress/BI_CarryPlayer.LiftToHook`
  (bind _asbp_hook (cast `/Game/Blueprint/Hook/BP_Hook` (`|GetArrayItem` (`PrimitiveComponent.GetOverlappingActors` (`self.CapsuleComponent`) "/Game/Blueprint/Hook/BP_Hook.BP_Hook_C"))))
  (`self.K2_AttachToComponent` _asbp_hook null "None" "SnapToTarget" "SnapToTarget" "KeepRelative" true)
  (set `self.PlayerStatee` "NewEnumerator16")
  (if (< (`self.HookNum`) 3)
    (message `/Game/Blueprint/Hook/BI_HookAction.DeadPlayer` _asbp_hook self)))

(fn `UserConstructionScript`)