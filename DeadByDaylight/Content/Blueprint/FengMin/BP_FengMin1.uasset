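; BP_FengMin1 is a playable character with Enhanced Input movement, look and run, plus a two-hit injury system.
; Running raises walk speed and sets a player state enum.
; GetAttacked first marks the character injured with a brief speed burst above run speed, then on later hits switches to a faint state with faint speed and query-only FaintCollision.
; It also caches default speed at BeginPlay and stores an assigned player ID.
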(event `self.ReceiveBeginPlay`
  ; 시작 시 스피드 설정 및 콜리젼
  (set `self.DefaultSpeed` (`CharacterMovementComponent.MaxWalkSpeed` (`self.CharacterMovement`)))
  (`PrimitiveComponent.SetCollisionEnabled` (`self.FaintCollision`) "NoCollision"))

(event `EnhancedInput|/Game/Blueprint/Controller/IA_Rotation`
  (params (ActionValue :type "Vector2D Structure") (ElapsedSeconds :type "Float (double-precision)") (TriggeredSeconds :type "Float (double-precision)") (InputAction :type "InputAction Object Reference" :default "/Game/Blueprint/Controller/IA_Rotation.IA_Rotation"))
  ; Rotation
  (:`Triggered`
    (`self.AddControllerYawInput` ActionValue_X)
    (`self.AddControllerPitchInput` ActionValue_Y)))

(event `SetPlayerId`
  (params (Id :type Integer))
  (set `self.PlayerId` Id))

(event `EnhancedInput|/Game/Blueprint/Controller/IA_Move`
  (params (ActionValue :type "Vector2D Structure") (ElapsedSeconds :type "Float (double-precision)") (TriggeredSeconds :type "Float (double-precision)") (InputAction :type "InputAction Object Reference" :default "/Game/Blueprint/Controller/IA_Move.IA_Move"))
  (bind (_returnvalue_roll _returnvalue_pitch _returnvalue_yaw) (`KismetMathLibrary.BreakRotator` (`self.GetControlRotation`)))
  ; Movement
  (:`Triggered`
    (`self.AddMovementInput` (`KismetMathLibrary.GetRightVector` (`self.GetControlRotation`)) ActionValue_X)
    (`self.AddMovementInput` (`KismetMathLibrary.GetForwardVector` (`KismetMathLibrary.MakeRotator` 0.0 0.0 _returnvalue_yaw)) ActionValue_Y)))

(event `EnhancedInput|/Game/Blueprint/Controller/IA_Run`
  (params (ActionValue :type Boolean) (ElapsedSeconds :type "Float (double-precision)") (TriggeredSeconds :type "Float (double-precision)") (InputAction :type "InputAction Object Reference" :default "/Game/Blueprint/Controller/IA_Run.IA_Run"))
  ; Run
  (:`Triggered`
    (set `CharacterMovementComponent.MaxWalkSpeed` (`self.RunSpeed`) (`self.CharacterMovement`))
    (set `self.PlayerStatee` "NewEnumerator6")))

(event `GetAttacked`
  (bind _charactermovement (`self.CharacterMovement`))
  ; 공격 받은 후 로직 처리
  (if (`self.PlayerInjured`)
    (set `self.PlayerStatee` "NewEnumerator17")
    (set `CharacterMovementComponent.MaxWalkSpeed` (`self.FaintSpeed`) (`self.CharacterMovement`))
    (`PrimitiveComponent.SetCollisionEnabled` (`self.FaintCollision`) "QueryOnly")
    (else
      (set `self.PlayerInjured` true)
      (set `CharacterMovementComponent.MaxWalkSpeed` (* (`self.RunSpeed`) 1.3) _charactermovement)
      (`KismetSystemLibrary.Delay` 1.5)
      (set `CharacterMovementComponent.MaxWalkSpeed` (`self.RunSpeed`) _charactermovement))))

(fn `UserConstructionScript`)