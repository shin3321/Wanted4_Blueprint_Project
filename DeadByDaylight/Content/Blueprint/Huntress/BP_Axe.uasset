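; BP_Axe is the Huntress's axe, an actor that attacks BP_FengMin characters through its AttackCollision component.
; An overlap with BP_FengMin calls GetAttacked on that actor, then AttackEnd, and calls AttackBegin after a 1.5-second delay.
; AttackBegin and AttackEnd both set the collision to NoCollision, so neither event re-enables hit detection.
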(event `self.AttackCollision.OnComponentBeginOverlap`
  (params (OverlappedComponent :type "PrimitiveComponent Object Reference") (OtherActor :type "Actor Object Reference") (OtherComp :type "PrimitiveComponent Object Reference") (OtherBodyIndex :type Integer) (bFromSweep :type Boolean) (SweepResult :type "HitResult Structure (by ref)"))
  (bind _asbp_feng_min (cast `/Game/Blueprint/FengMin/BP_FengMin` OtherActor))
  (if true
    (`/Game/Blueprint/FengMin/BP_FengMin.GetAttacked` _asbp_feng_min)
    (`self.AttackEnd`)
    (`KismetSystemLibrary.Delay` 1.5)
    (`self.AttackBegin`)))

(event `AttackBegin`
  (`PrimitiveComponent.SetCollisionEnabled` (`self.AttackCollision`) "NoCollision"))

(event `AttackEnd`
  (`PrimitiveComponent.SetCollisionEnabled` (`self.AttackCollision`) "NoCollision"))

(fn `UserConstructionScript`)