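; BP_Huntress is the playable hunter character, which melees, throws axes and carries downed players to hooks.
; A HunterState value gates Enhanced Input actions, with delays and walk-speed changes timing the attack montage and projectile axe throw.
; Carrying calls Interact on BP_FengMin, and hook overlap or carry input calls LiftToHook.
; Non-locally controlled copies interpolate every tick toward externally set target location and rotation.
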(event `self.ReceiveTick`
  (params (DeltaSeconds :type "Float (single-precision)"))
  ; 움직임 recv
  (if (not (`self.IsLocallyControlled`))
    (`self.K2_SetActorLocation` (`KismetMathLibrary.VInterpTo` (`self.K2_GetActorLocation`) (`self.NewTargetLocation`) 0.0 1.0))
    (`self.K2_SetActorRotation` (`KismetMathLibrary.RInterpTo` (`self.K2_GetActorRotation`) (`self.NewTargetRotation`) 0.0 1.0))))

(event `self.ReceiveBeginPlay`
  (cast `/Game/Blueprint/Controller/BP_HunterController` (`self.GetController`))
  (set `self.DefaultSpeed` (`CharacterMovementComponent.MaxWalkSpeed` (`self.CharacterMovement`))))

(event `SetPlayerId`
  (params (Id :type Integer))
  (set `self.PlayerId` Id))

(event `EnhancedInput|/Game/Blueprint/Controller/IA_Rotation`
  (params (ActionValue :type "Vector2D Structure") (ElapsedSeconds :type "Float (double-precision)") (TriggeredSeconds :type "Float (double-precision)") (InputAction :type "InputAction Object Reference" :default "/Game/Blueprint/Controller/IA_Rotation.IA_Rotation"))
  ; Rotation
  (:`Triggered`
    (`self.AddControllerYawInput` ActionValue_X)
    (`self.AddControllerPitchInput` ActionValue_Y)))

(event `EnhancedInput|/Game/Blueprint/Controller/IA_Attack`
  (params (ActionValue :type Boolean) (ElapsedSeconds :type "Float (double-precision)") (TriggeredSeconds :type "Float (double-precision)") (InputAction :type "InputAction Object Reference" :default "/Game/Blueprint/Controller/IA_Attack.IA_Attack"))
  ; Attack
  (:`Triggered`
    (switch `/Game/Blueprint/Huntress/EHunterState` (`self.HunterState`)
      (:`NewEnumerator0`
        (set `self.HunterState` "NewEnumerator5")
        (`self.PlayAnimMontage` "/Game/Blueprint/Huntress/Animation/AM_HuntressAttack.AM_HuntressAttack")
        (set `CharacterMovementComponent.MaxWalkSpeed` 0.0 (`self.CharacterMovement`))
        (`KismetSystemLibrary.Delay` 1.5)
        (set `CharacterMovementComponent.MaxWalkSpeed` (`self.DefaultSpeed`) (`self.CharacterMovement`)))
      (:`NewEnumerator4`
        (set `self.HunterState` "NewEnumerator0")
        (set `CharacterMovementComponent.MaxWalkSpeed` (`self.DefaultSpeed`) (`self.CharacterMovement`))))))

(event `EnhancedInput|/Game/Blueprint/Controller/IA_Move`
  (params (ActionValue :type "Vector2D Structure") (ElapsedSeconds :type "Float (double-precision)") (TriggeredSeconds :type "Float (double-precision)") (InputAction :type "InputAction Object Reference" :default "/Game/Blueprint/Controller/IA_Move.IA_Move"))
  (bind (_returnvalue_roll _returnvalue_pitch _returnvalue_yaw) (`KismetMathLibrary.BreakRotator` (`self.GetControlRotation`)))
  ; Movement
  (:`Triggered`
    (switch `/Game/Blueprint/Huntress/EHunterState` (`self.HunterState`)
      (:`NewEnumerator0`
        _)
      (:`NewEnumerator3`
        _)
      (:`NewEnumerator4`
        _)
      (:`NewEnumerator6`
        _))
    (`self.AddMovementInput` (`KismetMathLibrary.GetRightVector` (`self.GetControlRotation`)) ActionValue_X)
    (`self.AddMovementInput` (`KismetMathLibrary.GetForwardVector` (`KismetMathLibrary.MakeRotator` 0.0 0.0 _returnvalue_yaw)) ActionValue_Y)))

(event `EnhancedInput|/Game/Blueprint/Controller/IA_Throw`
  (params (ActionValue :type Boolean) (ElapsedSeconds :type "Float (double-precision)") (TriggeredSeconds :type "Float (double-precision)") (InputAction :type "InputAction Object Reference" :default "/Game/Blueprint/Controller/IA_Throw.IA_Throw"))
  (bind _returnvalue_location (`KismetMathLibrary.BreakTransform` (`SceneComponent.GetSocketTransform` (`self.Mesh`) "PlayerCarrySocket" "RTS_World")))
  ; Throw
  (:`Started`
    (if (`|EnumEquality` (`self.HunterState`) "NewEnumerator0")
      (set `self.HunterState` "NewEnumerator3")
      (set `CharacterMovementComponent.MaxWalkSpeed` (* (`self.DefaultSpeed`) 0.7) (`self.CharacterMovement`))))
  (:`Completed`
    (set `self.HunterState` "NewEnumerator4")
    (`SceneComponent.SetHiddenInGame` (`self.Axe`) true false)
    (`KismetSystemLibrary.Delay` 0.8)
    (set `CharacterMovementComponent.MaxWalkSpeed` 0.0 (`self.CharacterMovement`))
    (bind _returnvalue (`|SpawnActorFromClass` "/Game/Blueprint/Huntress/BP_ProjectileAxe.BP_ProjectileAxe_C" (`KismetMathLibrary.MakeTransform` (+ _returnvalue_location (20.0 50.0 80.0)) (struct :`Yaw` 90.0) (2.0 2.0 2.0)) "Undefined" "MultiplyWithRoot" null null))
    (set `MovementComponent.Velocity` (+ (* (`KismetMathLibrary.GetForwardVector` (`SceneComponent.K2_GetComponentRotation` (`self.Camera`))) 5000) (+ (`self.GetActorUpVector`) 500)) (`/Game/Blueprint/Huntress/BP_ProjectileAxe.ProjectileMovement` _returnvalue))
    (`KismetSystemLibrary.Delay` 1.5)
    (set `CharacterMovementComponent.MaxWalkSpeed` (`self.DefaultSpeed`) (`self.CharacterMovement`))
    (set `self.HunterState` "NewEnumerator0")
    (`SceneComponent.SetHiddenInGame` (`self.Axe`) false false)))

(event `AttackEnd`
  (set `self.HunterState` "NewEnumerator0"))

(event `UpPlayer`
  (set `self.CanCarry` true))

(event `EnhancedInput|/Game/Blueprint/Controller/IA_Carry`
  (params (ActionValue :type Boolean) (ElapsedSeconds :type "Float (double-precision)") (TriggeredSeconds :type "Float (double-precision)") (InputAction :type "InputAction Object Reference" :default "/Game/Blueprint/Controller/IA_Carry.IA_Carry"))
  (:`Triggered`
    (switch `/Game/Blueprint/Huntress/EHunterState` (`self.HunterState`)
      (:`NewEnumerator0`
        ; 플레이어 옮기기
        (if (`self.CanCarry`)
          (set `self.HunterState` "NewEnumerator6")
          (`SceneComponent.SetVisibility` (`self.Axe`) false false)
          (bind _asbp_feng_min (cast `/Game/Blueprint/FengMin/BP_FengMin` (`self.CarryOnPlayer`)))
          (`/Game/Blueprint/FengMin/BP_FengMin.Interact` _asbp_feng_min (`self.Mesh`))))
      (:`NewEnumerator6`
        ; 갈고리
        (cast `/Game/Blueprint/Hook/BP_Hook` (`|GetArrayItem` (`PrimitiveComponent.GetOverlappingActors` (`self.HookCollision`) "/Game/Blueprint/Hook/BP_Hook.BP_Hook_C")))
        (if true
          (`/Game/Blueprint/Huntress/BI_CarryPlayer.LiftToHook` (`self.CarryOnPlayer`)))))))

(event `self.HookCollision.OnComponentBeginOverlap`
  (params (OverlappedComponent :type "PrimitiveComponent Object Reference") (OtherActor :type "Actor Object Reference") (OtherComp :type "PrimitiveComponent Object Reference") (OtherBodyIndex :type Integer) (bFromSweep :type Boolean) (SweepResult :type "HitResult Structure (by ref)"))
  ; 갈고리
  (cast `/Game/Blueprint/Hook/BP_Hook` OtherActor)
  (if true
    (`/Game/Blueprint/Huntress/BI_CarryPlayer.LiftToHook` (`self.CarryOnPlayer`))))

(fn `UserConstructionScript`)